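; Player dash component that launches player character 0 when the dash input fires, with a one-second delay before it can dash again.
; Dash launches along the last movement input, or along the first-person camera's horizontal forward components when there is none.
; It zeroes ground friction and braking before the launch and restores fixed values immediately afterward in the same execution, with no delay.
; The input-driven branch also prints the input vector.
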(event Input|EnhancedActionEvents|EnhancedInputActionIA_Dash
  (params (ActionValue :type Boolean) (ElapsedSeconds :type Float%20%28double-precision%29) (TriggeredSeconds :type Float%20%28double-precision%29) (InputAction :type Input%20Action%20Object%20Reference :default "/Game/Movement/IA_Dash.IA_Dash"))
  (CallFunction|Dash)
  (Utilities|FlowControl|Delay 1.0)
  (Variables|Default|SetCan%20Dash true)
  (Variables|Default|SetIsDashing false))

(fn Dash
  (bind _returnvalue (Game|GetPlayerCharacter 0))
  (bind _returnvalue_2 (Game|GetPlayerCharacter 0))
  (bind _returnvalue_3 (Game|GetPlayerCharacter 0))
  (bind _returnvalue_4 (Game|GetPlayerCharacter 0))
  (bind _charactermovement (Variables|/Script/Engine.Character|GetCharacterMovement _returnvalue_3))
  (bind _charactermovement_2 (Variables|/Script/Engine.Character|GetCharacterMovement _returnvalue_2))
  (bind _charactermovement_3 (Variables|/Script/Engine.Character|GetCharacterMovement _returnvalue_4))
  (bind _returnvalue_5 (Pawn|Components|PawnMovement|GetLastInputVector _charactermovement_2))
  (if (Variables|Default|GetCan%20Dash)
    (Variables|Default|SetIsDashing true)
    (Variables|Default|SetCan%20Dash false)
    (Variables|/Script/Engine.CharacterMovementComponent|SetGroundFriction _charactermovement_3 0.0)
    (Variables|/Script/Engine.CharacterMovementComponent|SetBrakingFrictionFactor _charactermovement_3 0.0)
    (Variables|/Script/Engine.CharacterMovementComponent|SetBrakingDecelerationWalking _charactermovement_3 0.0)
    (if (Utilities|Operators|EqualEqual :A _returnvalue_5)
      (bind _asbp_first_person_character (Utilities|Casting|CastToBP_FirstPersonCharacter _returnvalue))
      (Character|LaunchCharacter _returnvalue (* (Math|Vector|GetForwardVector (Variables|/Game/FirstPerson/Blueprints/BP_FirstPersonCharacter.BP_FirstPersonCharacter_C|GetFirstPersonCamera _asbp_first_person_character)) "2000.000000,2000.000000,0.000000") false false)
      (else
        (Development|PrintString (Utilities|String|ToString(Vector) _returnvalue_5))
        (Character|LaunchCharacter (Game|GetPlayerCharacter 0) (* _returnvalue_5 2e+03) false false)))
    (Variables|/Script/Engine.CharacterMovementComponent|SetGroundFriction _charactermovement 8.0)
    (Variables|/Script/Engine.CharacterMovementComponent|SetBrakingFrictionFactor _charactermovement 2.0)
    (Variables|/Script/Engine.CharacterMovementComponent|SetBrakingDecelerationWalking _charactermovement 2048.0)))