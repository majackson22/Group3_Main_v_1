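; BP_StaticEnemy1 is an enemy that damages the player on contact and is destroyed if the player is dashing.
; Its Hit event passes a DoOnce, checks for BP_FirstPersonCharacter, then reads the player's dash component.
; Without a dash it lowers health through BPC_HealthAndDamage and resets the gate after a short delay.
; A hit from any other actor consumes the gate without resetting it.
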(event Collision|EventHit
  (params (MyComp :type Primitive%20Component%20Object%20Reference) (Other :type Actor%20Object%20Reference) (OtherComp :type Primitive%20Component%20Object%20Reference) (bSelfMoved :type Boolean) (HitLocation :type Vector :default "0, 0, 0") (HitNormal :type Vector :default "0, 0, 0") (NormalImpulse :type Vector :default "0, 0, 0") (Hit :type Hit%20Result%20Structure%20%28by%20ref%29))
  (bind _returnvalue (Game|GetPlayerCharacter 0))
  (Utilities|FlowControl|DoOnce false :!label _label
    (:Completed
      (Development|PrintString "Enemy collided with something.")
      (if (== (Utilities|GetClass Other) "/Game/FirstPerson/Blueprints/BP_FirstPersonCharacter.BP_FirstPersonCharacter_C")
        (Development|PrintString "Collided with player")
        (Variables|Default|SetHaD (Actor|GetComponentbyClass _returnvalue "/Game/HealthAndDamage/BPC_HealthAndDamage.BPC_HealthAndDamage_C"))
        (bind _output_get (Variables|Default|SetDash (Actor|GetComponentbyClass _returnvalue "/Game/Movement/BPC_PlayerDash.BPC_PlayerDash_C")))
        (if (Variables|/Game/Movement/BPC_PlayerDash.BPC_PlayerDash_C|GetIsDashing _output_get)
          (Development|PrintString "Enemy is dead")
          (Actor|DestroyActor)
          (else
            (Default|DecreaseHealth (Variables|Default|GetHaD) 2e+01)
            (Utilities|FlowControl|Delay 1.0)
            (goto _label Reset)))))))

(fn ConstructionScript)